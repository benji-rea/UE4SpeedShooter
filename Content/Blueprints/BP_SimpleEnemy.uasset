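; Simple enemy that chases the speed shooter player character and shows a health bar widget bound to itself.
; Pawn sensing starts an AI move toward the seen player while the enemy is alive.
; Projectile hits apply fixed damage and send it after the player, with no death check.
; Tick polls the dead flag to hide the health bar.
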(event `self.ReceiveBeginPlay`
  (bind _asenemy_health_bar (cast `/Game/Widgets/EnemyHealthBar` (`WidgetComponent.GetUserWidgetObject` (`self.HealthBar`))))
  (set `/Game/Widgets/EnemyHealthBar.HealthBarOwner` self _asenemy_health_bar))

(event `self.ReceiveHit`
  (params (MyComp :type "PrimitiveComponent Object Reference") (Other :type "Actor Object Reference") (OtherComp :type "PrimitiveComponent Object Reference") (bSelfMoved :type Boolean) (HitLocation :type "Vector Structure") (HitNormal :type "Vector Structure") (NormalImpulse :type "Vector Structure") (Hit :type "HitResult Structure (by ref)"))
  (cast `Projectile` Other)
  (`self.TakeDamage` 0.3)
  (bind _asbp_speed_shooter_character (cast `/Game/Blueprints/BP_SpeedShooterCharacter` (`GameplayStatics.GetPlayerCharacter` 0)))
  (`|AIMoveTo` self (0.0 0.0 0.0) _asbp_speed_shooter_character))

(event `self.ReceiveTick`
  (params (DeltaSeconds :type "Float (single-precision)"))
  (if (`self.isDead`)
    (`SceneComponent.SetVisibility` (`self.HealthBar`) false false)))

(event `self.PawnSensing.OnSeePawn`
  (params (Pawn :type "Pawn Object Reference"))
  (if (not (`self.isDead`))
    (bind _asbp_speed_shooter_character (cast `/Game/Blueprints/BP_SpeedShooterCharacter` Pawn))
    (`|AIMoveTo` self (0.0 0.0 0.0) _asbp_speed_shooter_character)))

(fn `UserConstructionScript`)