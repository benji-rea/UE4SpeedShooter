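; Player character Blueprint for a speed shooter, handling weapon setup, weapon mesh swapping and a fire sound.
; BeginPlay spawns an FPS weapon actor at the character's transform, stores it in the Weapons array and sets the default projectile class.
; SwitchWeaponMesh swaps the skeletal mesh between AR4 and SMG11 by index, with both using the same simple ammo.
; Releasing Fire only plays a laser sound at the weapon; no projectile spawning happens in this graph.
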(event `self.SwitchWeaponMesh`
  (params (_index :type Integer))
  (switch `int` _index
    (:`0`
      (`SkinnedMeshComponent.SetSkinnedAssetAndUpdate` (`self.PlayerWeapon`) "/Game/FPS_Weapon_Bundle/Weapons/Meshes/AR4/SK_AR4_X.SK_AR4_X" true)
      (set `self.ProjectileClass` "/Game/Blueprints/Weapons/Ammo/BP_SimpleAmmo.BP_SimpleAmmo_C"))
    (:`1`
      (`SkinnedMeshComponent.SetSkinnedAssetAndUpdate` (`self.PlayerWeapon`) "/Game/FPS_Weapon_Bundle/Weapons/Meshes/SMG11/SK_SMG11_Nostock_X.SK_SMG11_Nostock_X" true)
      (set `self.ProjectileClass` "/Game/Blueprints/Weapons/Ammo/BP_SimpleAmmo.BP_SimpleAmmo_C"))))

(event `self.ReceiveBeginPlay`
  (bind _returnvalue (`|SpawnActorFromClass` "/Game/Blueprints/Weapons/BP_FPSWeapon.BP_FPSWeapon_C" (`self.GetTransform`) "AdjustIfPossibleButAlwaysSpawn" "OverrideRootScale" null null))
  (set `self.Weapons` (`|MakeArray` _returnvalue :!type "FPSWeapon Object Reference"))
  (set `self.ProjectileClass` "/Game/Blueprints/Weapons/Ammo/BP_SimpleAmmo.BP_SimpleAmmo_C"))

(event `InputAction|Fire`
  (params (Key :type "Key Structure"))
  (:`Released`
    (`GameplayStatics.PlaySoundAtLocation` "/Engine/VREditor/Sounds/UI/Laser_Push.Laser_Push" (`SceneComponent.K2_GetComponentLocation` (`self.PlayerWeapon`)) (struct) 1.0 1.0 0.0 null null null)))

(fn `UserConstructionScript`)